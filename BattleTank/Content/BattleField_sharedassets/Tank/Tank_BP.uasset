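; Player tank pawn that drives, aims, fires and switches between first- and third-person cameras.
; On BeginPlay it passes barrel, turret and tracks to the TankAiming and TankMovement components, then links itself to its health bar widget.
; Input forwards movement intents and firing to those components.
; Camera axes rotate a gimbal for yaw and the spring arm for pitch, scaled by delta time.
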(event EventBeginPlay
  (Class|TankAimingComponent|SetAiming (Variables|Default|GetTankAiming) (Variables|Default|GetBarrel) (Variables|Default|GetTurret))
  (Class|TankMovementComponent|SetTracks (Variables|Default|GetTankMovement) (Variables|Default|GetLeftTrack) (Variables|Default|GetRightTrack))
  (bind _ashealth_bar (Utilities|Casting|CastToHealthBar (UserInterface|GetUserWidgetObject (Variables|Default|GetHealthBar%20Holder))))
  (Variables|/Game/UI/HealthBar.HealthBar_C|SetTank _ashealth_bar self))

(event Input|ActionEvents|InputActionFire
  (params (Key :type Key%20Structure :default "AnyKey"))
  (:Pressed
    (Class|TankAimingComponent|Fire (Variables|Default|GetTankAiming))))

(event Input|ActionEvents|InputActionChangeCamera
  (params (Key :type Key%20Structure :default "AnyKey"))
  (:Pressed
    (Components|Activation|ToggleActive (Variables|Default|Get1st%20Person))
    (Components|Activation|ToggleActive (Variables|Default|Get3rd%20Person))))

(event Input|AxisEvents|InputAxisHorizontal
  (params (AxisValue :type Float%20%28single-precision%29))
  ;[1 1 1] Camera Yaw
  (Transformation|AddLocalRotation (Variables|Default|GetHorizontal%20Gimbal) (Math|Rotator|MakeRotator 0.0 0.0 (* AxisValue (Utilities|Time|GetWorldDeltaSeconds) 5e+01)) false false))

(event Input|AxisEvents|InputAxisVertical
  (params (AxisValue :type Float%20%28single-precision%29))
  ;[1 1 1] Camera Pitch
  (Transformation|AddLocalRotation (Variables|Default|GetSpringArm) (Math|Rotator|MakeRotator 0.0 (* AxisValue (Utilities|Time|GetWorldDeltaSeconds) 5e+01) 0.0) false false))

(event Input|AxisEvents|InputAxisMoveForward
  (params (AxisValue :type Float%20%28single-precision%29))
  ;[1 1 1] Movement
  (Class|TankMovementComponent|IntendMoveForward (Variables|Default|GetTankMovement) AxisValue))

(event Input|AxisEvents|InputAxisTurn
  (params (AxisValue :type Float%20%28single-precision%29))
  ;[1 1 1] Movement
  (Class|TankMovementComponent|IntendTurn (Variables|Default|GetTankMovement) AxisValue))

(fn ConstructionScript)